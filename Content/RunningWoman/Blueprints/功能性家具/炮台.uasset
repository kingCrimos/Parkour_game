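; Cannon turret Blueprint (炮台) that fires projectiles continuously for as long as it is in play.
; BeginPlay calls the fire event, which spawns a shell actor (子弹) at the FirePoint transform and applies an impulse to its 炮弹 component along FirePoint's up vector, scaled by a launch-force variable.
; The event then re-arms a non-looping timer on itself using the interval variable, with no targeting or stop condition.
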(event `持续发射炮弹`
  (bind `_炮弹发射力度` (`self.炮弹发射力度`))
  (bind _firepoint (`self.FirePoint`))
  (bind _returnvalue (`|SpawnActorFromClass` "/Game/RunningWoman/Blueprints/功能性家具/子弹.子弹_C" (`KismetMathLibrary.MakeTransform` (`SceneComponent.K2_GetComponentLocation` _firepoint) (`SceneComponent.K2_GetComponentRotation` _firepoint)) "Undefined" "OverrideRootScale" null null))
  (`PrimitiveComponent.AddImpulse` (`/Game/RunningWoman/Blueprints/功能性家具/子弹.炮弹` _returnvalue) (* (`SceneComponent.GetUpVector` _firepoint) (`KismetMathLibrary.MakeVector` `_炮弹发射力度` `_炮弹发射力度` `_炮弹发射力度`)) "None" false)
  (`KismetSystemLibrary.K2_SetTimerDelegate` (delegate `持续发射炮弹`) (`self.炮弹发射间隔时间`)))

(event `self.ReceiveBeginPlay`
  (`self.持续发射炮弹`))

(fn `UserConstructionScript`)