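; Breakable furniture actor that knocks the third-person character back on each hit and shatters on the fourth.
; Box hits increment a counter and call the character's 被击退 with a scaled backward-and-upward vector.
; The breaking hit enables Geometry Collection physics and applies a radial external cluster strain field sized by the Sphere, with no falloff.
; It also knocks the character back, removes the Box and destroys the actor three seconds later.
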(event `self.ReceiveBeginPlay`
  (set `self.碰撞次数` 0)
  (`PrimitiveComponent.SetSimulatePhysics` (`self.破坏_GeometryCollection`) false))

(event `self.Box.OnComponentHit`
  (params (HitComponent :type "PrimitiveComponent Object Reference") (OtherActor :type "Actor Object Reference") (OtherComp :type "PrimitiveComponent Object Reference") (NormalImpulse :type "Vector Structure") (Hit :type "HitResult Structure (by ref)"))
  (bind `_击退倍数` (`self.击退倍数`))
  (bind _sphere (`self.Sphere`))
  (bind _asbp_third_person_character (cast `/Game/RunningWoman/Blueprints/BP_ThirdPersonCharacter` OtherActor))
  (if (>= (`self.碰撞次数`) 3)
    (`/Engine/EditorBlueprintResources/StandardMacros.DoOnce` false
      (:`Completed`
        (`PrimitiveComponent.SetSimulatePhysics` (`self.破坏_GeometryCollection`) true)
        (`FieldSystemComponent.ApplyPhysicsField` (`self.FieldSystem`) true "Field_ExternalClusterStrain" null (`RadialFalloff.SetRadialFalloff` (`self.RadialFalloff`) (`self.Field Magnitude`) 0.0 1.0 0.0 (`SphereComponent.GetScaledSphereRadius` _sphere) (`SceneComponent.K2_GetComponentLocation` _sphere) "Field_FallOff_None"))
        (`|ExecutionSequence`
          (:`then_0`
            (bind (_returnvalue_x _returnvalue_y) (`KismetMathLibrary.BreakVector` (`SceneComponent.GetForwardVector` (`Actor.RootComponent` _asbp_third_person_character))))
            (`/Game/RunningWoman/Blueprints/BP_ThirdPersonCharacter.被击退` _asbp_third_person_character (* (* (`KismetMathLibrary.MakeVector` _returnvalue_x _returnvalue_y 1.0) (-10000.0 -10000.0 10000.0)) (`KismetMathLibrary.MakeVector` `_击退倍数` `_击退倍数` `_击退倍数`)) :!label _label))
          (:`then_1`
            (`ActorComponent.K2_DestroyComponent` (`self.Box`))
            (`KismetSystemLibrary.Delay` 3.0)
            (`self.K2_DestroyActor`)))))
    (else
      (set `self.碰撞次数` (+ (`self.碰撞次数`) 1))
      (goto _label))))

(fn `UserConstructionScript`)