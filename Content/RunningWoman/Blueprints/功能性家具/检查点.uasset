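; Checkpoint actor that records a respawn point on the player's third-person character.
; When a BP_ThirdPersonCharacter begins overlapping the Box, it writes the Root's world location, raised slightly on Z, and world rotation into the character's checkpoint position and angle variables.
; The checkpoint then destroys itself, so each placed instance triggers only once.
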(event `self.Box.OnComponentBeginOverlap`
  (params (OverlappedComponent :type "PrimitiveComponent Object Reference") (OtherActor :type "Actor Object Reference") (OtherComp :type "PrimitiveComponent Object Reference") (OtherBodyIndex :type Integer) (bFromSweep :type Boolean) (SweepResult :type "HitResult Structure (by ref)"))
  (bind _root (`self.Root`))
  (bind _asbp_third_person_character (cast `/Game/RunningWoman/Blueprints/BP_ThirdPersonCharacter` OtherActor))
  (set `/Game/RunningWoman/Blueprints/BP_ThirdPersonCharacter.检查点位置` (`KismetMathLibrary.MakeVector` (.x (`SceneComponent.K2_GetComponentLocation` _root)) (.y (`SceneComponent.K2_GetComponentLocation` _root)) (+ (.z (`SceneComponent.K2_GetComponentLocation` _root)) 100.0)) _asbp_third_person_character)
  (set `/Game/RunningWoman/Blueprints/BP_ThirdPersonCharacter.检查点角度` (`SceneComponent.K2_GetComponentRotation` _root) _asbp_third_person_character)
  (`self.K2_DestroyActor` self))

(fn `UserConstructionScript`)