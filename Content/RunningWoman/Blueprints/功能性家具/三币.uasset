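; A coin pickup actor that bobs and spins until the third-person character collects it.
; On BeginPlay one timeline moves Root up and down along Z, and each update plays or reverses a second timeline that drives yaw rotation, with direction chosen by the 正反 flag.
; Overlapping the Box with BP_ThirdPersonCharacter calls its 吃到金币 function with a value of three, then destroys the coin.
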(event `self.ReceiveBeginPlay`
  ;[1 1 1] 上下位移
  (bind (_direction `_新建轨道_0`) (`Timeline|时间轴_0`)
    (:`Update`
      (`SceneComponent.K2_SetRelativeLocation` (`self.Root`) (`KismetMathLibrary.MakeVector` 0.0 0.0 (`KismetMathLibrary.Lerp` 0.0 30.0 `_新建轨道_0`)) false false)
      ;[1 1 1] 旋转
      (if (`self.正反`)
        (bind (_direction_2 `_新建轨道_0_2`) (`Timeline|时间轴_1` :!label _label)
          (:`Update`
            (`SceneComponent.K2_SetRelativeRotation` (`self.DefaultSceneRoot`) (`KismetMathLibrary.MakeRotator` 0.0 0.0 `_新建轨道_0_2`) false false)))
        (else
          (goto _label :!via `Reverse`))))))

(event `self.Box.OnComponentBeginOverlap`
  (params (OverlappedComponent :type "PrimitiveComponent Object Reference") (OtherActor :type "Actor Object Reference") (OtherComp :type "PrimitiveComponent Object Reference") (OtherBodyIndex :type Integer) (bFromSweep :type Boolean) (SweepResult :type "HitResult Structure (by ref)"))
  (bind _asbp_third_person_character (cast `/Game/RunningWoman/Blueprints/人物/BP_ThirdPersonCharacter` OtherActor))
  (`/Game/RunningWoman/Blueprints/人物/BP_ThirdPersonCharacter.吃到金币` _asbp_third_person_character 3)
  (`self.K2_DestroyActor`))

(fn `UserConstructionScript`)