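; Knockback actor in the functional furniture folder that launches the player away when touched, then destroys itself.
; A timeline started on BeginPlay moves the root vertically through a Z lerp.
; Box overlap with BP_ThirdPersonCharacter fires once, calling its 被击退 (knocked back) function with a force pointing horizontally away from the box plus a fixed upward component, scaled by the 击退倍数 multiplier.
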(event `self.ReceiveBeginPlay`
  ;[1 1 1] 上下位移
  (bind (_direction `_新建轨道_0`) (`Timeline|时间轴_1`)
    (:`Update`
      (`SceneComponent.K2_SetRelativeLocation` (`self.Root`) (`KismetMathLibrary.MakeVector` 0.0 0.0 (`KismetMathLibrary.Lerp` 0.0 50.0 `_新建轨道_0`)) false false))))

(event `self.Box.OnComponentBeginOverlap`
  (params (OverlappedComponent :type "PrimitiveComponent Object Reference") (OtherActor :type "Actor Object Reference") (OtherComp :type "PrimitiveComponent Object Reference") (OtherBodyIndex :type Integer) (bFromSweep :type Boolean) (SweepResult :type "HitResult Structure (by ref)"))
  (bind `_击退倍数` (`self.击退倍数`))
  ;[1 1 1] 击退
  (bind _asbp_third_person_character (cast `/Game/RunningWoman/Blueprints/人物/BP_ThirdPersonCharacter` OtherActor))
  (`/Engine/EditorBlueprintResources/StandardMacros.DoOnce` false
    (:`Completed`
      (bind (_returnvalue_x _returnvalue_y) (`KismetMathLibrary.BreakVector` (`KismetMathLibrary.GetDirectionUnitVector` (`SceneComponent.K2_GetComponentLocation` (`self.Box`)) (`SceneComponent.K2_GetComponentLocation` (`Actor.RootComponent` _asbp_third_person_character)))))
      (`/Game/RunningWoman/Blueprints/人物/BP_ThirdPersonCharacter.被击退` _asbp_third_person_character (* (* (`KismetMathLibrary.MakeVector` _returnvalue_x _returnvalue_y 1.0) (10000.0 10000.0 10000.0)) (`KismetMathLibrary.MakeVector` `_击退倍数` `_击退倍数` `_击退倍数`)))
      (`self.K2_DestroyActor`))))

(fn `UserConstructionScript`)